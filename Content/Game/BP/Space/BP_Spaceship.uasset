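; Player-controlled spaceship Blueprint that thrusts along its up vector while the fly input is held.
; BeginPlay adds the Enhanced Input mapping context, and IA_Fly toggles the flying flag and starts or stops a DoOnce-gated engine sound.
; Tick applies physics force while alive and flying, activates a Niagara effect when not alive, and spawns warp effects during a dash, clearing that flag after a delay.
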(event Custom|Add%20Force%20Up
  (bind _spaceship (Variables|Default|GetSpaceship))
  ;[1 1 1] Force Up Spaceship
  (Physics|AddForce _spaceship (* (Math|Vector|GetUpVector _spaceship) (Variables|Default|GetfForce)) "None" false))

(event Input|EnhancedActionEvents|EnhancedInputActionIA_Fly
  (params (ActionValue :type Boolean) (ElapsedSeconds :type Float%20%28double-precision%29) (TriggeredSeconds :type Float%20%28double-precision%29) (InputAction :type Input%20Action%20Object%20Reference :default "/Game/Game/PlayerInput/Input_Action/IA_Fly.IA_Fly"))
  ;[1 1 1] Vérif si le joueur clique sur Fly
  (:Started
    (Variables|Default|SetbIsFlying true :!label _label)
    (Utilities|FlowControl|DoOnce false :!label _label_2
      (:Completed
        (bind _returnvalue (Audio|SpawnSound2D "/Game/Game/Audio/SFX/vaisseau_qui_monte_v3.vaisseau_qui_monte_v3" 1.0 1.0 0.0 0))
        (Variables|Default|SetAudioSpaceship _returnvalue))))
  (:Ongoing
    (goto _label))
  (:Canceled
    (Variables|Default|SetbIsFlying false :!label _label_3)
    (Utilities|FlowControl|Sequence
      (:then_0
        (goto _label_2 Reset))
      (:then_1
        (Audio|Components|Audio|Stop (Variables|Default|GetAudioSpaceship)))))
  (:Completed
    (goto _label_3)))

(event EventTick
  (params (DeltaSeconds :type Float%20%28single-precision%29))
  (bind _spaceship (Variables|Default|GetSpaceship))
  (bind _returnvalue (Transformation|GetRelativeTransform _spaceship))
  ;[1 1 1] Tick
  (Utilities|FlowControl|Sequence
    (:then_0
      (if (Variables|Default|GetIsAlive)
        (if (Variables|Default|GetbIsFlying)
          (CallFunction|AddForceUp))
        (else
          (Components|Activation|Activate (Variables|Default|GetNiagara) false))))
    (:then_1
      (if (Variables|Default|GetIsDash)
        (Niagara|SpawnSystematLocation "/Game/Game/asset/Niagara/NS_Warp.NS_Warp" (- (.location _returnvalue) "0.000000,0.000000,100.000000") (.rotation _returnvalue) "100.000000,0.000000,30.000000")
        (Utilities|FlowControl|Delay 1.0)
        (Variables|Default|SetIsDash false)))))

(event EventBeginPlay
  ;[1 1 1] Récupère IMC
  (bind _asplayer_controller (Utilities|Casting|CastToPlayerController (Pawn|GetController)))
  (Utilities|IsValid (PlayerController|LocalPlayerSubsystems|GetEnhancedInputLocalPlayerSubsystem _asplayer_controller)
    (:Is%20Valid
      (Input|AddMappingContext (PlayerController|LocalPlayerSubsystems|GetEnhancedInputLocalPlayerSubsystem _asplayer_controller) "/Game/Game/PlayerInput/IMC_PlayerMouvement.IMC_PlayerMouvement" 1 "(bIgnoreAllPressedKeysUntilRelease=True,bForceImmediately=False,bNotifyUserSettings=False)"))))

(fn ConstructionScript)