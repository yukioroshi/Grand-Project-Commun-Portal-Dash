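; Manager for the snow level that builds spline terrain tiles as play progresses and ends the run on death.
; It spawns two starting tiles plus generation and killzone actors, which it moves along the track.
; Generation collider overlaps, gated by DoOnce nodes, drive tile spawning and removal until the tile count triggers a portal on the last tile.
; Killzone or obstacle deaths show the end screen and clear tile tracking.
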(event Custom|KillPlayer
  (params (OverlappedActor :type Actor%20Object%20Reference) (OtherActor :type Actor%20Object%20Reference))
  ;[1 1 1] Comment
  (if (Variables|/Game/Game/BP/Snow/BP_SnowKillzone.BP_SnowKillzone_C|GetKillPlayer (Variables|Default|GetKillBox))
    (bind _returnvalue (Game|ConstructObjectfromClass "/Game/Game/BP/UI/UI_EndScreen.UI_EndScreen_C"))
    (UserInterface|Viewport|AddtoViewport _returnvalue 0)
    (Utilities|Array|Clear (Variables|Default|GetGenerated%20Tiles))
    (Utilities|Array|Clear (Variables|Default|Get3/4Mark%20Point%20Transform))
    (Utilities|Array|Clear (Variables|Default|GetEnd%20Points%20Transform))))

(event Custom|CreateTerrain
  (params (OverlappedActor :type Actor%20Object%20Reference) (OtherActor :type Actor%20Object%20Reference))
  (bind _generated_tiles (Variables|Default|GetGenerated%20Tiles))
  ;[1 1 1] Comment
  (Utilities|FlowControl|DoOnce true
    (:Completed
      (if (Variables|/Game/Game/BP/Snow/BP_SnowGenerationCollider.BP_SnowGenerationCollider_C|GetGenerateNewTerrain (Variables|Default|GetGenerationManagerBP))
        (if (> (Utilities|Array|Length _generated_tiles) 2)
          (Utilities|FlowControl|Sequence
            (:then_0
              _)
            (:then_1
              (Utilities|FlowControl|Delay 2.0)
              (Actor|DestroyActor (Utilities|Array|Get(acopy) _generated_tiles))
              (Utilities|Array|RemoveIndex _generated_tiles))))
        (CallFunction|SpawnSplineBP)))))

(event Custom|SpawnSplineBP
  (bind _generated_tiles (Variables|Default|GetGenerated%20Tiles))
  ;[1 1 1] Comment
  (Transformation|SetActorLocation (Variables|Default|GetGenerationManagerBP) (+ (.Location (Math|Transform|BreakTransform (Variables|Default|GetStart%20Spawn%20Transform))) "0.000000,0.000000,15000.000000") false true)
  (Transformation|SetActorLocation (Variables|Default|GetKillBox) (- (.Location (Math|Transform|BreakTransform (Variables|Default|GetStart%20Spawn%20Transform))) "0.000000,40000.000000,1000.000000") false true)
  (Utilities|FlowControl|DoOnce false
    (:Completed
      (if (>= (Variables|Default|GetNumberOFTilesSpawned) 4)
        (bind _asbp_snow_terrain_generation (Utilities|Casting|CastToBP_SnowTerrainGeneration (Utilities|Array|Get(acopy) _generated_tiles (Utilities|Array|LastIndex _generated_tiles))))
        (Default|GeneratePortal _asbp_snow_terrain_generation)
        (else
          (bind _returnvalue (Game|SpawnActorfromClass "/Game/Game/BP/Snow/BP_SnowTerrainGeneration.BP_SnowTerrainGeneration_C" (Variables|Default|GetStart%20Spawn%20Transform) "Undefined" "MultiplyWithRoot" 0 0))
          (Utilities|FlowControl|Sequence
            (:then_0
              (Utilities|Array|Add (Variables|Default|GetGenerated%20Tiles) _returnvalue)
              (Utilities|Array|Add (Variables|Default|GetEnd%20Points%20Transform) (Variables|/Game/Game/BP/Snow/BP_SnowTerrainGeneration.BP_SnowTerrainGeneration_C|GetSplineLastPos _returnvalue))
              (Utilities|Array|Add (Variables|Default|Get3/4Mark%20Point%20Transform) (Variables|/Game/Game/BP/Snow/BP_SnowTerrainGeneration.BP_SnowTerrainGeneration_C|Get3/4%20Mark _returnvalue))
              (bind _result (Math|Integer|IncrementInt (Variables|Default|GetNumberOFTilesSpawned))
                (:%20%20
                  (Variables|Default|SetNumberOFTilesSpawned _result))))
            (:then_1
              (Variables|Default|SetStart%20Spawn%20Transform (Math|Transform|MakeTransform (+ (Variables|/Game/Game/BP/Snow/BP_SnowTerrainGeneration.BP_SnowTerrainGeneration_C|GetSplineLastPos _returnvalue) "0.000000,100.000000,-200.000000")))
              (Variables|/Game/Game/BP/Snow/BP_SnowGenerationCollider.BP_SnowGenerationCollider_C|SetGenerateNewTerrain (Variables|Default|GetGenerationManagerBP) false))))))))

(event Custom|Reset
  (params (OverlappedActor :type Actor%20Object%20Reference) (OtherActor :type Actor%20Object%20Reference))
  (bind _generated_tiles (Variables|Default|GetGenerated%20Tiles))
  (bind _generated_tiles_2 (Variables|Default|GetGenerated%20Tiles))
  ;[1 1 1] Comment
  (Utilities|FlowControl|Delay 2.0)
  (Utilities|FlowControl|Sequence
    (:then_0
      ;[1 1 1] Comment
      (Utilities|FlowControl|DoOnce true) ; enters at Reset
    )
    (:then_1
      (Utilities|FlowControl|DoOnce false) ; enters at Reset
    )))

(event Custom|ObstacleKillPlayer
  ;[1 1 1] Comment
  (bind _returnvalue (Game|ConstructObjectfromClass "/Game/Game/BP/UI/UI_EndScreen.UI_EndScreen_C"))
  (UserInterface|Viewport|AddtoViewport _returnvalue 0)
  (Utilities|Array|Clear (Variables|Default|GetGenerated%20Tiles))
  (Utilities|Array|Clear (Variables|Default|Get3/4Mark%20Point%20Transform))
  (Utilities|Array|Clear (Variables|Default|GetEnd%20Points%20Transform)))

(event EventBeginPlay
  ;[1 1 1] Comment
  (Variables|Default|SetIsSnowPlaying true)
  (Utilities|FlowControl|Sequence
    (:then_0
      (EventDispatchers|UnbindallEventsfromOnActorBeginOverlap)
      (EventDispatchers|UnbindallEventsfromOnActorEndOverlap))
    (:then_1
      (bind _returnvalue (Game|SpawnActorfromClass "/Game/Game/BP/Snow/BP_SnowGenerationCollider.BP_SnowGenerationCollider_C" (Math|Conversions|ToTransform(Vector) (+ (.Location (Math|Transform|BreakTransform (Variables|Default|GetStart%20Spawn%20Transform))) "0.000000,5000.000000,5000.000000")) "Undefined" "MultiplyWithRoot" 0 0))
      (Variables|Default|SetGenerationManagerBP _returnvalue)
      (bind _returnvalue_2 (Game|SpawnActorfromClass "/Game/Game/BP/Snow/BP_SnowKillzone.BP_SnowKillzone_C" (Math|Conversions|ToTransform(Vector) (+ (.Location (Math|Transform|BreakTransform (Variables|Default|GetStart%20Spawn%20Transform))) "0.000000,5000.000000,5000.000000")) "Undefined" "MultiplyWithRoot" 0 0))
      (Variables|Default|SetKillBox _returnvalue_2)
      (Utilities|FlowControl|DelayUntilNextTick)
      (Variables|Default|SetIsStart true)
      (Utilities|FlowControl|Sequence
        (:then_0
          (Collision|BindEventtoOnActorBeginOverlap (Variables|Default|GetGenerationManagerBP) (delegate Custom|CreateTerrain))
          (Collision|BindEventtoOnActorEndOverlap (Variables|Default|GetGenerationManagerBP) (delegate Custom|Reset)))
        (:then_1
          (Utilities|FlowControl|DoOnce false
            (:Completed
              (for _index (range 0 1)
                (bind _returnvalue_3 (Game|SpawnActorfromClass "/Game/Game/BP/Snow/BP_SnowTerrainGeneration.BP_SnowTerrainGeneration_C" (Variables|Default|GetStart%20Spawn%20Transform) "Undefined" "MultiplyWithRoot" 0 0))
                (Utilities|FlowControl|Sequence
                  (:then_0
                    (Utilities|Array|Add (Variables|Default|GetGenerated%20Tiles) _returnvalue_3)
                    (Utilities|Array|Add (Variables|Default|GetEnd%20Points%20Transform) (Variables|/Game/Game/BP/Snow/BP_SnowTerrainGeneration.BP_SnowTerrainGeneration_C|GetSplineLastPos _returnvalue_3))
                    (Utilities|Array|Add (Variables|Default|Get3/4Mark%20Point%20Transform) (Variables|/Game/Game/BP/Snow/BP_SnowTerrainGeneration.BP_SnowTerrainGeneration_C|Get3/4%20Mark _returnvalue_3))
                    (bind _result (Math|Integer|IncrementInt (Variables|Default|GetNumberOFTilesSpawned))
                      (:%20%20
                        (Variables|Default|SetNumberOFTilesSpawned _result))))
                  (:then_1
                    (Variables|Default|SetStart%20Spawn%20Transform (Math|Transform|MakeTransform (+ (Variables|/Game/Game/BP/Snow/BP_SnowTerrainGeneration.BP_SnowTerrainGeneration_C|GetSplineLastPos _returnvalue_3) "0.000000,100.000000,-200.000000")))
                    (Utilities|FlowControl|DoOnce false
                      (:Completed
                        (Variables|/Game/Game/BP/Snow/BP_SnowGenerationCollider.BP_SnowGenerationCollider_C|SetGenerateNewTerrain (Variables|Default|GetGenerationManagerBP) false)
                        (Transformation|SetActorLocation (Variables|Default|GetGenerationManagerBP) (+ (Variables|/Game/Game/BP/Snow/BP_SnowTerrainGeneration.BP_SnowTerrainGeneration_C|GetSplineLastPos _returnvalue_3) "0.000000,0.000000,15000.000000") false true)
                        (Transformation|SetActorLocation (Variables|Default|GetKillBox) (- (Variables|/Game/Game/BP/Snow/BP_SnowTerrainGeneration.BP_SnowTerrainGeneration_C|GetSplineLastPos _returnvalue_3) "0.000000,40000.000000,1500.000000") false true)
                        (Variables|Default|SetIsStart false)))))))))
        (:then_2
          (Collision|BindEventtoOnActorBeginOverlap (Variables|Default|GetKillBox) (delegate Custom|KillPlayer)))))))

(event EventDestroyed
  (Variables|Default|SetIsSnowPlaying false))

(fn ConstructionScript)