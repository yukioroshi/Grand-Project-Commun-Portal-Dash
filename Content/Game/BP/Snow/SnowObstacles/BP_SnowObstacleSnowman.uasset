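; Snowman obstacle for the snow game that is either smashed by a fast player or kills a slow one.
; On the first box overlap with BP_SnowPlayer, it prints the player's velocity and tests the Y component against a speed threshold.
; Above it, the player's physics velocity is zeroed, SpeedCheckWait runs and the snowman is destroyed.
; Otherwise, after a short delay, BP_SnowGameManager's ObstacleKillPlayer is called.
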(event OnComponentBeginOverlap(Box)
  (params (OverlappedComponent :type Primitive%20Component%20Object%20Reference) (OtherActor :type Actor%20Object%20Reference) (OtherComp :type Primitive%20Component%20Object%20Reference) (OtherBodyIndex :type Integer) (bFromSweep :type Boolean) (SweepResult :type Hit%20Result%20Structure%20%28by%20ref%29))
  (bind _asbp_snow_player (Utilities|Casting|CastToBP_SnowPlayer OtherActor))
  (Utilities|FlowControl|DoOnce false
    (:Completed
      (Development|PrintText (Utilities|Text|ToText(String) (Transformation|GetVelocity _asbp_snow_player)) true true "(R=1.000000,G=0.000000,B=0.186585,A=1.000000)" 15.0)
      (if (> (.Y (Math|Vector|BreakVector (Transformation|GetVelocity _asbp_snow_player))) 1.2e+03)
        (Physics|SetPhysicsLinearVelocity (Variables|/Game/Game/BP/Snow/BP_SnowPlayer.BP_SnowPlayer_C|Getportaldash_3d_snow_character _asbp_snow_player) "0, 0, 0" false "None")
        (Default|SpeedCheckWait _asbp_snow_player)
        (Actor|DestroyActor)
        (else
          (bind _returnvalue (Actor|GetActorOfClass "/Game/Game/BP/Snow/BP_SnowGameManager.BP_SnowGameManager_C"))
          (Utilities|FlowControl|Delay 0.2)
          (Default|ObstacleKillPlayer _returnvalue))))))

(event EventBeginPlay)

(event Collision|EventActorBeginOverlap
  (params (OtherActor :type Actor%20Object%20Reference)))

(event EventTick
  (params (DeltaSeconds :type Float%20%28single-precision%29)))

(fn ConstructionScript)