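; Physics-driven player pawn for the snow level, with hold-to-jump, a glider and timed glider and wine power-ups.
; Terrain hits and a downward trace drive the grounded and can-glide states that gate jumping and gliding.
; Enhanced Input applies jump and glide forces, while Tick nudges Y speed into range and widens camera FOV with speed.
; Power-up timers count down on Tick and report to the GameInstance UI, which is cleared on destruction.
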(event OnComponentHit(portaldash_3d_snow_character)
  (params (HitComponent :type Primitive%20Component%20Object%20Reference) (OtherActor :type Actor%20Object%20Reference) (OtherComp :type Primitive%20Component%20Object%20Reference) (NormalImpulse :type Vector :default "0, 0, 0") (Hit :type Hit%20Result%20Structure%20%28by%20ref%29))
  ;[1 1 1] Ground Check
  (Utilities|Casting|CastToBP_SnowTerrainGeneration OtherActor)
  (Variables|Default|SetRayEnabled true)
  (bind _output_get (Variables|Default|SetisGrouded true))
  (if _output_get
    (Variables|Default|SetCanGlide false)
    (Utilities|FlowControl|RetriggerableDelay 0.3)
    (Variables|Default|SetRayEnabled false)
    (Variables|Default|SetisGrouded false)
    (else
      (Variables|Default|SetCanGlide true))))

(event Custom|Ground%20Check
  (bind _portaldash_3d_snow_character (Variables|Default|Getportaldash_3d_snow_character))
  (bind _returnvalue (Transformation|GetWorldLocation _portaldash_3d_snow_character))
  ;[1 1 1] Raycast for leaving the ground
  (if (Variables|Default|GetRayEnabled)
    (bind _returnvalue_2 (Collision|LineTraceByChannel _returnvalue (+ _returnvalue (* (Variables|Default|GetRayLenght) (* (Math|Vector|GetUpVector (Transformation|GetWorldRotation _portaldash_3d_snow_character)) -1.0))) "TraceTypeQuery1" false 0 "ForOneFrame"))
    (if (and _returnvalue_2 (not (Variables|Default|GetIsJumping)))
      (Variables|Default|SetCanGlide false)
      (else
        (Variables|Default|SetisGrouded _returnvalue_2)
        (Variables|Default|SetCanGlide true)))))

(event Custom|WineTick
  ;[1 1 1] Wine Tick
  (Variables|Default|SetCurrentWineTimer (Math|Float|Clamp(Float) (- (Variables|Default|GetCurrentWineTimer) (Utilities|Time|GetWorldDeltaSeconds)) 0.0 (Variables|Default|GetCurrentWineTimer)))
  (Default|UpdatePowerUpTime (Variables|Default|GetGameInstance) (Math|Float|Round (Variables|Default|GetCurrentWineTimer)))
  (if (<= (Variables|Default|GetCurrentWineTimer) 0.0)
    (Rendering|SetVisibility (Variables|Default|Getportaldash_3d_snow_wine) false false)
    (Variables|Default|SetHasWine false)))

(event Custom|GliderTick
  ;[1 1 1] Glider Tick
  (Variables|Default|SetCurrentGliderTimer (Math|Float|Clamp(Float) (- (Variables|Default|GetCurrentGliderTimer) (Utilities|Time|GetWorldDeltaSeconds)) 0.0 (Variables|Default|GetCurrentGliderTimer)))
  (Default|UpdatePowerUpTime (Variables|Default|GetGameInstance) (Math|Float|Round (Variables|Default|GetCurrentGliderTimer)))
  (if (<= (Variables|Default|GetCurrentGliderTimer) 0.0)
    (Variables|Default|SetHasGlider false)))

(event Custom|FOVTick
  (bind _camera (Variables|Default|GetCamera))
  ;[1 1 1] Change FOV depending of speed
  (if (> (.Y (Math|Vector|BreakVector (Transformation|GetVelocity))) 1.4e+03)
    (Variables|Default|SetFOVBlend (Math|Vector|DotProduct (Math|Conversions|ToVector(Float) (.Y (Math|Vector|BreakVector (Math|Vector|Normalize (Transformation|GetVelocity))))) (Math|Conversions|ToVector(Float) (.Y (Math|Vector|BreakVector (Transformation|GetActorForwardVector))))))
    (else
      (Variables|Default|SetFOVBlend 0.0)))
  (Camera|SetFieldOfView _camera (Math|Float|Clamp(Float) (Math|Interpolation|FInterptoConstant (Variables|/Script/Engine.CameraComponent|GetFieldOfView _camera) (Math|Float|Lerp (Variables|Default|GetDefaultFOV) (Variables|Default|GetFastFOV) (Variables|Default|GetFOVBlend)) (Utilities|Time|GetWorldDeltaSeconds) (Variables|Default|GetFOVSpeedBlend)) 9e+01 1.2e+02)))

(event Custom|SpeedTick
  (bind _returnvalue (Transformation|GetVelocity))
  (bind _isgliding (Variables|Default|GetIsGliding))
  (bind _portaldash_3d_snow_character (Variables|Default|Getportaldash_3d_snow_character))
  (bind _isgrouded (Variables|Default|GetisGrouded))
  (bind _y (Math|Vector|BreakVector _returnvalue))
  (bind _returnvalue_2 (or _isgrouded _isgliding))
  ;[1 1 1] PlayerSpeedCheck
  (if (Variables|Default|GetCanSpeedCheck)
    (Utilities|FlowControl|Sequence
      (:then_0
        (if (and (> _y 2.6e+03) _returnvalue_2)
          (Physics|SetPhysicsLinearVelocity _portaldash_3d_snow_character "0.000000,-20.000000,0.000000" true "None")))
      (:then_1
        (if (and (< _y 7e+02) _returnvalue_2)
          (Physics|SetPhysicsLinearVelocity _portaldash_3d_snow_character "0.000000,20.000000,0.000000" true "None"))))))

(event Custom|SpeedCheckWait
  ;[1 1 1] Speed Check delay
  (Variables|Default|SetCanSpeedCheck false)
  (Utilities|FlowControl|RetriggerableDelay 0.5)
  (Variables|Default|SetCanSpeedCheck true))

(event Custom|WineCollect
  ;[1 1 1] Collect Wine
  (Variables|Default|SetHasWine true)
  (Variables|Default|SetCurrentWineTimer (Variables|Default|GetWineTimer))
  (Rendering|SetVisibility (Variables|Default|Getportaldash_3d_snow_wine) true false)
  (Default|PowerUpUI (Variables|Default|GetGameInstance) 2 (Math|Float|Round (Variables|Default|GetWineTimer))) ; 0=Shield\n1=Laser\n2=Wine\n3=Glider\n4=Lasso
)

(event Custom|GliderCollected
  (bind _glidertimer (Variables|Default|GetGliderTimer))
  ;[1 1 1] Glider Colection
  (Variables|Default|SetHasGlider true)
  (Audio|PlaySound2D 0 1.0 1.0 0.0 0 0)
  (Variables|Default|SetCurrentGliderTimer _glidertimer)
  (Variables|Default|SetGlider%20Reset false)
  (Default|PowerUpUI (Variables|Default|GetGameInstance) 3 (Math|Float|Truncate _glidertimer)) ; 0=Shield\n1=Laser\n2=Wine\n3=Glider\n4=Lasso
)

(event Input|EnhancedActionEvents|EnhancedInputActionIA_Slider
  (params (ActionValue :type Boolean) (ElapsedSeconds :type Float%20%28double-precision%29) (TriggeredSeconds :type Float%20%28double-precision%29) (InputAction :type Input%20Action%20Object%20Reference :default "/Game/Game/PlayerInput/Input_Action/IA_Slider.IA_Slider"))
  ;[1 1 1] Jump Depending of time pressed
  (:Ongoing
    (Utilities|FlowControl|Sequence
      (:then_0
        (if (Variables|Default|GetisGrouded)
          (if (> 0.4 ElapsedSeconds)
            (Physics|AddForce (Variables|Default|Getportaldash_3d_snow_character) (Variables|Default|GetImpulse%20Force) "None" true)
            (else
              (Variables|Default|SetIsJumping false)
              (Variables|Default|SetisGrouded false)
              (Variables|Default|SetCanGlide true)))))
      (:then_1
        (Utilities|FlowControl|DoOnce false
          (:Completed
            (if (Variables|Default|GetisGrouded)
              (Variables|Default|SetIsJumping true)
              (else
                (Variables|Default|SetIsJumping false))))))))
  (:Canceled
    (Variables|Default|SetIsJumping false :!label _label)
    (Variables|Default|SetisGrouded false)
    (Variables|Default|SetCanGlide true))
  (:Completed
    (goto _label)))

(event Input|EnhancedActionEvents|EnhancedInputActionIA_Glider
  (params (ActionValue :type Boolean) (ElapsedSeconds :type Float%20%28double-precision%29) (TriggeredSeconds :type Float%20%28double-precision%29) (InputAction :type Input%20Action%20Object%20Reference :default "/Game/Game/PlayerInput/Input_Action/IA_Glider.IA_Glider"))
  (bind _portaldash_3d_snow_character (Variables|Default|Getportaldash_3d_snow_character))
  (bind _portaldash_3d_snow_character_2 (Variables|Default|Getportaldash_3d_snow_character))
  (bind _portaldash_3d_snow_character_3 (Variables|Default|Getportaldash_3d_snow_character))
  (bind _returnvalue (Physics|GetPhysicsAngularVelocityinDegrees _portaldash_3d_snow_character_3 "None"))
  (bind _x (Math|Vector|BreakVector _returnvalue))
  ;[1 1 1] Glider Logic
  (:Ongoing
    (if (not (Variables|Default|GetisGrouded))
      (if (Variables|Default|GetHasGlider)
        (if (Variables|Default|GetCanGlide)
          (if (<= (Math|Vector|DotProduct (Math|Vector|Normalize (Transformation|GetComponentVelocity _portaldash_3d_snow_character) 0.1) (Math|Vector|GetUpVector _portaldash_3d_snow_character)) 0.0)
            (Utilities|FlowControl|Sequence
              (:then_0
                (bind _output_get (Variables|Default|SetIsGliding true))
                (Rendering|SetVisibility (Variables|Default|Getportaldash_3d_snow_glider) _output_get false)
                (bind _returnvalue_2 (Audio|SpawnSound2D "/Game/Game/Audio/SFX/planeur_sound_effect.planeur_sound_effect" 1.0 1.0 0.0 0))
                (Variables|Default|SetAudioGlider _returnvalue_2)
                (Physics|AddForce (Variables|Default|Getportaldash_3d_snow_character) (Variables|Default|GetGliderThrust) "None" true))
              (:then_1
                (if (!= _x 0.0)
                  (Utilities|FlowControl|Sequence
                    (:then_0
                      (if (< _x 0.0)
                        (Class|PrimitiveComponent|SetPhysicsAngularVelocityinDegrees _portaldash_3d_snow_character_2 "0.500000,0.000000,-0.000000" true "None")))
                    (:then_1
                      (if (not (> _x 0.0))
                        (Class|PrimitiveComponent|SetPhysicsAngularVelocityinDegrees _portaldash_3d_snow_character_2 "-0.500000,0.000000,0.000000" true "None")))
                    (:then_2
                      (if (== _x 0.0)
                        (Class|PrimitiveComponent|SetPhysicsAngularVelocityinDegrees _portaldash_3d_snow_character_2 "0, 0, 0" false "None"))))))))))))
  (:Canceled
    (if (and (Variables|Default|GetIsGliding) (Variables|Default|GetHasGlider)) :!label _label
      (bind _output_get_2 (Variables|Default|SetIsGliding false))
      (Rendering|SetVisibility (Variables|Default|Getportaldash_3d_snow_glider) _output_get_2 false)
      (Audio|Components|Audio|Stop (Variables|Default|GetAudioGlider))))
  (:Completed
    (goto _label)))

(event EventDestroyed
  ;[1 1 1] Hide HUD if PowerUp is done sooner
  (bind _asbp_game_instance (Utilities|Casting|CastTobp_GameInstance (Game|GetGameInstance)))
  (Default|PowerUpDone _asbp_game_instance))

(event EventBeginPlay
  ;[1 1 1] Get MappingContext
  (bind _asplayer_controller (Utilities|Casting|CastToPlayerController (Pawn|GetController)))
  (Utilities|IsValid (PlayerController|LocalPlayerSubsystems|GetEnhancedInputLocalPlayerSubsystem _asplayer_controller)
    (:Is%20Valid
      (Input|AddMappingContext (PlayerController|LocalPlayerSubsystems|GetEnhancedInputLocalPlayerSubsystem _asplayer_controller) "/Game/Game/PlayerInput/IMC_PlayerMouvement.IMC_PlayerMouvement" 1 "(bIgnoreAllPressedKeysUntilRelease=True,bForceImmediately=False,bNotifyUserSettings=False)")
      (CallFunction|SpeedCheckWait)
      (bind _asbp_game_instance (Utilities|Casting|CastTobp_GameInstance (Game|GetGameInstance)))
      (Variables|Default|SetGameInstance _asbp_game_instance))))

(event EventTick
  (params (DeltaSeconds :type Float%20%28single-precision%29))
  ;[1 1 1] Tick
  (CallFunction|GroundCheck)
  (Utilities|FlowControl|Sequence
    (:then_0
      (if (Variables|Default|GetHasGlider)
        (CallFunction|GliderTick)))
    (:then_1
      (CallFunction|FOVTick))
    (:then_2
      (if (or (Variables|Default|GetisGrouded) (Variables|Default|GetIsGliding))
        (CallFunction|SpeedTick)))
    (:then_3
      (if (Variables|Default|GetHasWine)
        (CallFunction|WineTick)))))

(fn ConstructionScript)