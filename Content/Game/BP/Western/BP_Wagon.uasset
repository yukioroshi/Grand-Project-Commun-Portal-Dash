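; Player wagon for a Western level, switching between three lanes through vertical swipes or Left/Right keys.
; A timeline lerps the wagon and any active lasso between lane positions while re-pinning the camera in world space.
; Collider overlaps show the end screen on obstacles, spawn TNT and an explosion, or start a timed lasso.
; The Game Instance drives the power-up HUD, updated each tick during the lasso and cleared on destruction.
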(event OnComponentBeginOverlap(Player_collider)
  (params (OverlappedComponent :type Primitive%20Component%20Object%20Reference) (OtherActor :type Actor%20Object%20Reference) (OtherComp :type Primitive%20Component%20Object%20Reference) (OtherBodyIndex :type Integer) (bFromSweep :type Boolean) (SweepResult :type Hit%20Result%20Structure%20%28by%20ref%29))
  (bind _body (Variables|Default|GetBody))
  (bind _body_2 (Variables|Default|GetBody))
  (bind _body_3 (Variables|Default|GetBody))
  (bind _lassoinitialtimer (Variables|Default|GetLassoInitialTimer))
  (bind _returnvalue (Transformation|GetWorldLocation _body))
  (bind _returnvalue_2 (Transformation|GetWorldLocation _body_2))
  (bind _returnvalue_3 (Transformation|GetWorldLocation _body_3))
  ;[1 1 1] collision with power UP and obstacle
  (Utilities|FlowControl|Sequence
    (:then_0
      ;;[1 1 1] condition de mort
      (Utilities|Casting|CastTobp_ObstacleWestern OtherActor)
      (Utilities|FlowControl|Delay 0.1)
      (bind _returnvalue_4 (Game|ConstructObjectfromClass "/Game/Game/BP/UI/UI_EndScreen.UI_EndScreen_C"))
      (UserInterface|Viewport|AddtoViewport _returnvalue_4 0))
    (:then_1
      ;;[1 1 1] Activate TNT
      (Utilities|Casting|CastToBP_TNTobject OtherActor)
      (bind _returnvalue_5 (Game|SpawnActorfromClass "/Game/Game/BP/PowerUps/BP_TNT.BP_TNT_C" (Math|Transform|MakeTransform (Math|Vector|MakeVector (.x _returnvalue_3) (.y _returnvalue_3) (+ (.z _returnvalue_3) 2e+01)) "0, 0, 0" "1.000000,2.000000,1.000000") "Undefined" "MultiplyWithRoot" 0 0))
      (Actor|SetLifeSpan _returnvalue_5 0.4)
      (Game|SpawnActorfromClass "/Game/Game/asset/PowerUp/TNT/Explosion/BP_Explosion.BP_Explosion_C" (Math|Transform|MakeTransform (Math|Vector|MakeVector (.x _returnvalue_2) (Variables|Default|GetInitialPos) (.z _returnvalue_2)) "0, 0, 0" "1.000000,2.000000,1.000000") "Undefined" "MultiplyWithRoot" 0 0))
    (:then_2
      ;;[1 1 1] Activate Lasso
      (Utilities|Casting|CastToBP_Lasso OtherActor)
      (if (not (Variables|Default|GetLassoActive))
        (bind _returnvalue_6 (Game|SpawnActorfromClass "/Game/Game/BP/PowerUps/BP_ActiveLasso.BP_ActiveLasso_C" (Math|Transform|MakeTransform (Math|Vector|MakeVector (.x _returnvalue) (.y _returnvalue) 28.0) "0, 0, 0" "1.000000,1.000000,1.000000") "Undefined" "MultiplyWithRoot" 0 0))
        (Variables|Default|SetActiveLasso _returnvalue_6)
        (Variables|Default|SetLassoActive true)
        (Rendering|SetVisibility (Variables|Default|GetLasso) true false)
        (bind _returnvalue_7 (Audio|SpawnSound2D "/Game/Game/Audio/SFX/lasso_en_cours_utilisation_2.lasso_en_cours_utilisation_2" 1.0 1.0 0.0 0))
        (Variables|Default|SetAudioLasso _returnvalue_7)
        (Variables|Default|SetCurrentLassoTimer _lassoinitialtimer)
        (Default|PowerUpUI (Variables|Default|GetGameInstance) 4 (Math|Float|Truncate _lassoinitialtimer)) ; 0=Shield\n1=Laser\n2=Wine\n3=Glider\n4=Lasso
      ))))

(event Custom|Check_Swiping
  (bind _returnvalue (Game|GetPlayerController 0))
  (bind _lane_y (Variables|Default|GetLane%20Y))
  (bind _lane_z (Variables|Default|GetLane%20Z))
  (bind _body (Variables|Default|GetBody))
  (bind _returnvalue_2 (Transformation|GetWorldLocation _body))
  (bind (_locationx _locationy) (Class|PlayerController|GetInputTouchState _returnvalue "Touch1"))
  ;[1 1 1] swiping up and down
  (if (> (Math|Vector2D|Vector2DLength (- (Variables|Default|GetTouchStart) (Variables|Default|GetTouchEnd))) 1e+02)
    (Utilities|FlowControl|DoOnce false
      (:Completed
        (Variables|Default|SetTouchEnd (Math|Vector2D|MakeVector2D _locationx _locationy))
        (if (> (Math|Float|Absolute(Float) (.X (Math|Vector2D|BreakVector2D (- (Variables|Default|GetTouchStart) (Variables|Default|GetTouchEnd))))) (Math|Float|Absolute(Float) (.Y (Math|Vector2D|BreakVector2D (- (Variables|Default|GetTouchStart) (Variables|Default|GetTouchEnd))))))
          (if (> (.X (Math|Vector2D|BreakVector2D (- (Variables|Default|GetTouchStart) (Variables|Default|GetTouchEnd)))) 0.0)
            _)
          (elif (> (.Y (Math|Vector2D|BreakVector2D (- (Variables|Default|GetTouchStart) (Variables|Default|GetTouchEnd)))) 0.0)
            ;[1 1 1] changing lanes
            (Utilities|FlowControl|Sequence
              (:then_0
                (Variables|Default|SetNewLane (Math|Integer|Clamp(Integer) (+ (Variables|Default|GetLane) -1) 0 2))
                (bind (_direction _lane_y_2 _lane_z_2) (Timeline|Chronologie PlayFromStart)
                  (:Update
                    (Transformation|SetActorLocation (Math|Vector|MakeVector (Math|Float|Lerp (Utilities|Array|Get(acopy) _lane_y (Variables|Default|GetLane)) (Utilities|Array|Get(acopy) _lane_y (Variables|Default|GetNewLane)) _lane_y_2) (.y _returnvalue_2) (Math|Float|Lerp (Utilities|Array|Get(acopy) _lane_z (Variables|Default|GetLane)) (Utilities|Array|Get(acopy) _lane_z (Variables|Default|GetNewLane)) _lane_z_2)) false false)
                    (Utilities|FlowControl|Sequence
                      (:then_0
                        ;[1 1 1] lasso keep player transform
                        (if (Variables|Default|GetLassoActive)
                          (bind _returnvalue_3 (Actor|GetActorOfClass "/Game/Game/BP/PowerUps/BP_ActiveLasso.BP_ActiveLasso_C"))
                          (bind _asbp_active_lasso (Utilities|Casting|CastToBP_ActiveLasso _returnvalue_3))
                          (Transformation|SetActorLocation _asbp_active_lasso (Math|Vector|MakeVector (Math|Float|Lerp (Utilities|Array|Get(acopy) _lane_y (Variables|Default|GetLane)) (Utilities|Array|Get(acopy) _lane_y (Variables|Default|GetNewLane)) _lane_y_2) (.y _returnvalue_2) (+ (Math|Float|Lerp (Utilities|Array|Get(acopy) _lane_z (Variables|Default|GetLane)) (Utilities|Array|Get(acopy) _lane_z (Variables|Default|GetNewLane)) _lane_z_2) 28.0)) false false)))
                      (:then_1
                        ;[1 1 1] set cam pos in world
                        (Transformation|SetWorldLocation (Variables|Default|GetCamera) (Math|Vector|MakeVector -3e+02 -1e+03 2e+02) false false)
                        (bind _asbp_game_instance (Utilities|Casting|CastTobp_GameInstance (Game|GetGameInstance)))
                        (Variables|Default|SetGameInstance _asbp_game_instance))))
                  (:Finished
                    (Variables|Default|SetLane (Variables|Default|GetNewLane))))))
            (else
              (Utilities|FlowControl|Sequence
                (:then_0
                  (Variables|Default|SetNewLane (Math|Integer|Clamp(Integer) (+ (Variables|Default|GetLane) 1) 0 2))
                  (Timeline|Chronologie PlayFromStart))))))))))

(event Custom|LassoTick
  ;[1 1 1] Lasso Tick
  (Variables|Default|SetCurrentLassoTimer (Math|Float|Clamp(Float) (- (Variables|Default|GetCurrentLassoTimer) (Utilities|Time|GetWorldDeltaSeconds)) 0.0 (Variables|Default|GetCurrentLassoTimer)))
  (Default|UpdatePowerUpTime (Variables|Default|GetGameInstance) (Math|Float|Round (Variables|Default|GetCurrentLassoTimer)))
  (if (<= (Variables|Default|GetCurrentLassoTimer) 0.0)
    (Variables|Default|SetLassoActive false)
    (Rendering|SetVisibility (Variables|Default|GetLasso) false false)
    (Audio|Components|Audio|Stop (Variables|Default|GetAudioLasso))
    (Actor|DestroyActor (Variables|Default|GetActiveLasso))))

(event EventBeginPlay
  ;[1 1 1] set cam pos in world
  (Transformation|SetWorldLocation (Variables|Default|GetCamera) (Math|Vector|MakeVector -3e+02 -1e+03 2e+02) false false)
  (bind _asbp_game_instance (Utilities|Casting|CastTobp_GameInstance (Game|GetGameInstance)))
  (Variables|Default|SetGameInstance _asbp_game_instance))

(event EventDestroyed
  ;[1 1 1] Hide HUD if PowerUp is done sooner
  (bind _asbp_game_instance (Utilities|Casting|CastTobp_GameInstance (Game|GetGameInstance)))
  (Default|PowerUpDone _asbp_game_instance))

(event EventTick
  (params (DeltaSeconds :type Float%20%28single-precision%29))
  ;[1 1 1] swiping up and down
  (Utilities|FlowControl|Sequence
    (:then_0
      (if (Variables|Default|GetLassoActive)
        (CallFunction|LassoTick)))
    (:then_1
      (if (Variables|Default|GetIsPressed)
        (CallFunction|CheckSwiping)))))

(event Input|KeyboardEvents|Right
  (params (Key :type Key%20Structure :default "None"))
  (bind _lane_y (Variables|Default|GetLane%20Y))
  (bind _lane_z (Variables|Default|GetLane%20Z))
  (bind _body (Variables|Default|GetBody))
  (bind _returnvalue (Transformation|GetWorldLocation _body))
  ;[1 1 1] changing lanes
  (:Pressed
    (Utilities|FlowControl|Sequence
      (:then_0
        (Variables|Default|SetNewLane (Math|Integer|Clamp(Integer) (+ (Variables|Default|GetLane) 1) 0 2))
        (bind (_direction _lane_y_2 _lane_z_2) (Timeline|Chronologie PlayFromStart)
          (:Update
            (Transformation|SetActorLocation (Math|Vector|MakeVector (Math|Float|Lerp (Utilities|Array|Get(acopy) _lane_y (Variables|Default|GetLane)) (Utilities|Array|Get(acopy) _lane_y (Variables|Default|GetNewLane)) _lane_y_2) (.y _returnvalue) (Math|Float|Lerp (Utilities|Array|Get(acopy) _lane_z (Variables|Default|GetLane)) (Utilities|Array|Get(acopy) _lane_z (Variables|Default|GetNewLane)) _lane_z_2)) false false)
            (Utilities|FlowControl|Sequence
              (:then_0
                ;[1 1 1] lasso keep player transform
                (if (Variables|Default|GetLassoActive)
                  (bind _returnvalue_2 (Actor|GetActorOfClass "/Game/Game/BP/PowerUps/BP_ActiveLasso.BP_ActiveLasso_C"))
                  (bind _asbp_active_lasso (Utilities|Casting|CastToBP_ActiveLasso _returnvalue_2))
                  (Transformation|SetActorLocation _asbp_active_lasso (Math|Vector|MakeVector (Math|Float|Lerp (Utilities|Array|Get(acopy) _lane_y (Variables|Default|GetLane)) (Utilities|Array|Get(acopy) _lane_y (Variables|Default|GetNewLane)) _lane_y_2) (.y _returnvalue) (+ (Math|Float|Lerp (Utilities|Array|Get(acopy) _lane_z (Variables|Default|GetLane)) (Utilities|Array|Get(acopy) _lane_z (Variables|Default|GetNewLane)) _lane_z_2) 28.0)) false false)))
              (:then_1
                ;[1 1 1] set cam pos in world
                (Transformation|SetWorldLocation (Variables|Default|GetCamera) (Math|Vector|MakeVector -3e+02 -1e+03 2e+02) false false)
                (bind _asbp_game_instance (Utilities|Casting|CastTobp_GameInstance (Game|GetGameInstance)))
                (Variables|Default|SetGameInstance _asbp_game_instance))))
          (:Finished
            (Variables|Default|SetLane (Variables|Default|GetNewLane))))))))

(event Input|KeyboardEvents|Left
  (params (Key :type Key%20Structure :default "None"))
  (bind _lane_y (Variables|Default|GetLane%20Y))
  (bind _lane_z (Variables|Default|GetLane%20Z))
  (bind _body (Variables|Default|GetBody))
  (bind _returnvalue (Transformation|GetWorldLocation _body))
  ;[1 1 1] changing lanes
  (:Pressed
    (Utilities|FlowControl|Sequence
      (:then_0
        (Variables|Default|SetNewLane (Math|Integer|Clamp(Integer) (+ (Variables|Default|GetLane) -1) 0 2))
        (bind (_direction _lane_y_2 _lane_z_2) (Timeline|Chronologie PlayFromStart)
          (:Update
            (Transformation|SetActorLocation (Math|Vector|MakeVector (Math|Float|Lerp (Utilities|Array|Get(acopy) _lane_y (Variables|Default|GetLane)) (Utilities|Array|Get(acopy) _lane_y (Variables|Default|GetNewLane)) _lane_y_2) (.y _returnvalue) (Math|Float|Lerp (Utilities|Array|Get(acopy) _lane_z (Variables|Default|GetLane)) (Utilities|Array|Get(acopy) _lane_z (Variables|Default|GetNewLane)) _lane_z_2)) false false)
            (Utilities|FlowControl|Sequence
              (:then_0
                ;[1 1 1] lasso keep player transform
                (if (Variables|Default|GetLassoActive)
                  (bind _returnvalue_2 (Actor|GetActorOfClass "/Game/Game/BP/PowerUps/BP_ActiveLasso.BP_ActiveLasso_C"))
                  (bind _asbp_active_lasso (Utilities|Casting|CastToBP_ActiveLasso _returnvalue_2))
                  (Transformation|SetActorLocation _asbp_active_lasso (Math|Vector|MakeVector (Math|Float|Lerp (Utilities|Array|Get(acopy) _lane_y (Variables|Default|GetLane)) (Utilities|Array|Get(acopy) _lane_y (Variables|Default|GetNewLane)) _lane_y_2) (.y _returnvalue) (+ (Math|Float|Lerp (Utilities|Array|Get(acopy) _lane_z (Variables|Default|GetLane)) (Utilities|Array|Get(acopy) _lane_z (Variables|Default|GetNewLane)) _lane_z_2) 28.0)) false false)))
              (:then_1
                ;[1 1 1] set cam pos in world
                (Transformation|SetWorldLocation (Variables|Default|GetCamera) (Math|Vector|MakeVector -3e+02 -1e+03 2e+02) false false)
                (bind _asbp_game_instance (Utilities|Casting|CastTobp_GameInstance (Game|GetGameInstance)))
                (Variables|Default|SetGameInstance _asbp_game_instance))))
          (:Finished
            (Variables|Default|SetLane (Variables|Default|GetNewLane))))))))

(event Input|TouchEvents|InputTouch
  (params (Location :type Vector) (FingerIndex :type ETouchIndex%20Enum))
  (bind (_x _y) (Math|Vector|BreakVector Location))
  (bind _returnvalue (Game|GetPlayerController 0))
  (bind _lane_y (Variables|Default|GetLane%20Y))
  (bind _lane_z (Variables|Default|GetLane%20Z))
  (bind _body (Variables|Default|GetBody))
  (bind _returnvalue_2 (Transformation|GetWorldLocation _body))
  (bind (_locationx _locationy) (Class|PlayerController|GetInputTouchState _returnvalue "Touch1"))
  ;[1 1 1] swiping up and down
  (:Pressed
    (Variables|Default|SetIsPressed true)
    (Variables|Default|SetTouchStart (Math|Vector2D|MakeVector2D _x _y)))
  (:Released
    (Variables|Default|SetTouchEnd (Math|Vector2D|MakeVector2D _x _y))
    (Utilities|FlowControl|DoOnce false) ; enters at Reset
  ))

(fn ConstructionScript)