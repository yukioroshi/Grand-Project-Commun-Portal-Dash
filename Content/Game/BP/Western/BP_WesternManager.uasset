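; Western level manager that spawns coins, power-ups and a portal from three spawner points.
; The self-repeating SpawnObstacle drops coins at one or two spawners, chosen by a Tick-randomized roll, with delays shrinking over game time.
; SpawnPowerUP places a lasso, TNT or shield pickup at random intervals, but stops looping on a roll of 3.
; A delayed Tick counter spawns the portal at Spawner1 upon reaching 50.
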(event Custom|spawn%20portal
  ;[1 1 1] Spawn Obstacle with Delay that decreased with the time
  (Development|PrintString "portal")
  (Game|SpawnActorfromClass "/Game/Game/BP/Portal/BP_WesternPortal.BP_WesternPortal_C" (Transformation|GetWorldTransform (Variables|Default|GetSpawner1)) "Undefined" "MultiplyWithRoot" 0 0))

(event Custom|SpawnPowerUP
  (bind _spawner (Variables|Default|GetSpawner))
  (bind _spawner1 (Variables|Default|GetSpawner1))
  (bind _spawner2 (Variables|Default|GetSpawner2))
  (bind _returnvalue (Transformation|GetWorldTransform _spawner1))
  (bind _returnvalue_2 (Transformation|GetWorldTransform _spawner2))
  (bind _returnvalue_3 (Transformation|GetWorldTransform _spawner))
  ;[1 1 1] Spawn Power UP
  (Utilities|FlowControl|Delay (Math|Random|RandomFloatinRange 1e+01 2e+01))
  (bind _output_get (Variables|Default|SetSelectedSpawn (Math|Random|RandomIntegerinRange 0 3)))
  (switch int _output_get
    (:0
      (switch int (Math|Random|RandomIntegerinRange 0 2)
        (:0
          (Game|SpawnActorfromClass "/Game/Game/BP/PowerUps/BP_Lasso.BP_Lasso_C" _returnvalue_3 "Undefined" "MultiplyWithRoot" 0 0))
        (:1
          (Game|SpawnActorfromClass "/Game/Game/BP/PowerUps/BP_TNTobject.BP_TNTobject_C" _returnvalue_3 "Undefined" "MultiplyWithRoot" 0 15.0 0))
        (:2
          (Game|SpawnActorfromClass "/Game/Game/BP/PowerUps/BP_RecupShield.BP_RecupShield_C" _returnvalue_3 "Undefined" "MultiplyWithRoot" 0 0)))
      (CallFunction|SpawnPowerUP))
    (:1
      (switch int (Math|Random|RandomIntegerinRange 0 2)
        (:0
          (Game|SpawnActorfromClass "/Game/Game/BP/PowerUps/BP_Lasso.BP_Lasso_C" _returnvalue "Undefined" "MultiplyWithRoot" 0 0))
        (:1
          (Game|SpawnActorfromClass "/Game/Game/BP/PowerUps/BP_TNTobject.BP_TNTobject_C" _returnvalue "Undefined" "MultiplyWithRoot" 0 15.0 0))
        (:2
          (Game|SpawnActorfromClass "/Game/Game/BP/PowerUps/BP_RecupShield.BP_RecupShield_C" _returnvalue "Undefined" "MultiplyWithRoot" 0 0)))
      (CallFunction|SpawnPowerUP))
    (:2
      (switch int (Math|Random|RandomIntegerinRange 0 2)
        (:0
          (Game|SpawnActorfromClass "/Game/Game/BP/PowerUps/BP_Lasso.BP_Lasso_C" _returnvalue_2 "Undefined" "MultiplyWithRoot" 0 0))
        (:1
          (Game|SpawnActorfromClass "/Game/Game/BP/PowerUps/BP_TNTobject.BP_TNTobject_C" _returnvalue_2 "Undefined" "MultiplyWithRoot" 0 15.0 0))
        (:2
          (Game|SpawnActorfromClass "/Game/Game/BP/PowerUps/BP_RecupShield.BP_RecupShield_C" _returnvalue_2 "Undefined" "MultiplyWithRoot" 0 0)))
      (CallFunction|SpawnPowerUP))))

(event Custom|Spawn%20Obstacle
  (bind _returnvalue (Utilities|Time|GetGameTimeinSeconds))
  (bind _returnvalue_2 (Math|Random|RandomInteger 0))
  (bind _ispawneractivate (Variables|Default|GetiSpawnerActivate))
  (bind _maxtime (Variables|Default|GetMaxTime))
  (bind _returnvalue_3 (Math|Float|MapRangeClamped _returnvalue 0.0 _maxtime 3.0 1.0))
  ;[1 1 1] Spawn Obstacle with Delay that decreased with the time
  (if (< _ispawneractivate 4)
    (Utilities|FlowControl|Delay _returnvalue_3 :!label _label)
    (switch int _returnvalue_2
      (:0
        (Game|SpawnActorfromClass "/Game/Game/BP/PowerUps/BP_Coin.BP_Coin_C" (Transformation|GetWorldTransform (Variables|Default|GetSpawner)) "Undefined" "MultiplyWithRoot" 0 0)))
    (elif (< _ispawneractivate 7)
      (Utilities|FlowControl|Delay _returnvalue_3 :!label _label_2)
      (switch int _returnvalue_2
        (:0
          (Game|SpawnActorfromClass "/Game/Game/BP/PowerUps/BP_Coin.BP_Coin_C" (Transformation|GetWorldTransform (Variables|Default|GetSpawner1)) "Undefined" "MultiplyWithRoot" 0 0)))
      (else
        (if (< _ispawneractivate 10)
          _
          (elif (== _ispawneractivate 10)
            (Utilities|FlowControl|Sequence
              (:then_0
                (goto _label))
              (:then_1
                (goto _label_2)))
            (elif (== _ispawneractivate 11)
              (Utilities|FlowControl|Sequence
                (:then_0
                  (goto _label_2))
                (:then_1
                  _))
              (else
                (Utilities|FlowControl|Sequence
                  (:then_0
                    (goto _label))
                  (:then_1
                    _))))))
        (Utilities|FlowControl|Delay _returnvalue_3)
        (switch int _returnvalue_2
          (:0
            (Game|SpawnActorfromClass "/Game/Game/BP/PowerUps/BP_Coin.BP_Coin_C" (Transformation|GetWorldTransform (Variables|Default|GetSpawner2)) "Undefined" "MultiplyWithRoot" 0 0))))))
  (CallFunction|SpawnObstacle))

(event EventBeginPlay
  ;[1 1 1] Call Obstacle on BeginPlay
  (Variables|Default|SetFRandomBegin (Math|Random|RandomFloatinRange 3.0 6.0))
  (Utilities|FlowControl|Delay 0.2)
  (CallFunction|SpawnObstacle)
  (CallFunction|SpawnPowerUP))

(event EventTick
  (params (DeltaSeconds :type Float%20%28single-precision%29))
  ;[1 1 1] Set wich spawner activate
  (Utilities|FlowControl|Sequence
    (:then_0
      (Variables|Default|SetiSpawnerActivate (Math|Random|RandomIntegerinRange 1 12)))
    (:then_1
      ;[1 1 1] when to spawn portal
      (Utilities|FlowControl|Delay 1.0)
      (bind _result (Math|Float|IncrementFloat (Variables|Default|GetDistanceOnBegin))
        (:%20%20
          (Variables|Default|SetDistanceOnBegin _result)
          ;[1 1 1] Spawn Obstacle with Delay that decreased with the time
          (if (>= (Variables|Default|GetDistanceOnBegin) 5e+01)
            (if (<= (Variables|Default|GetDistanceOnBegin) 50.1)
              (CallFunction|SpawnPortal))))))))

(fn ConstructionScript)