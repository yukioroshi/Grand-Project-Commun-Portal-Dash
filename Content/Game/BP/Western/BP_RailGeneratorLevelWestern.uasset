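; Rail generator for the Western level that repeatedly spawns BP_Rail_Western actors at three spawner components, starting on BeginPlay.
; SpawnRail uses a Sequence to spawn at each spawner, each branch followed by its own Delay that re-calls the whole event.
; The delay is mapped from game time against MaxTime, but both output bounds are equal, so the interval stays constant despite the comment saying it decreases.
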(event Custom|Spawn%20Rail
  (bind _returnvalue (Utilities|Time|GetGameTimeinSeconds))
  (bind _maxtime (Variables|Default|GetMaxTime))
  (bind _returnvalue_2 (Math|Float|MapRangeClamped _returnvalue 0.0 _maxtime 15.0 15.0))
  ;[1 1 1] Spawn Obstacle with Delay that decreased with the time
  (Utilities|FlowControl|Sequence
    (:then_0
      (Game|SpawnActorfromClass "/Game/Game/BP/Western/BP_Rail_Western.BP_Rail_Western_C" (Transformation|GetWorldTransform (Variables|Default|GetSpawner)) "Undefined" "MultiplyWithRoot" 0 0)
      (Utilities|FlowControl|Delay _returnvalue_2))
    (:then_1
      (Game|SpawnActorfromClass "/Game/Game/BP/Western/BP_Rail_Western.BP_Rail_Western_C" (Transformation|GetWorldTransform (Variables|Default|GetSpawner1)) "Undefined" "MultiplyWithRoot" 0 0)
      (Utilities|FlowControl|Delay _returnvalue_2))
    (:then_2
      (Game|SpawnActorfromClass "/Game/Game/BP/Western/BP_Rail_Western.BP_Rail_Western_C" (Transformation|GetWorldTransform (Variables|Default|GetSpawner2)) "Undefined" "MultiplyWithRoot" 0 0)
      (Utilities|FlowControl|Delay _returnvalue_2)))
  (CallFunction|SpawnRail))

(event EventBeginPlay
  ;[1 1 1] Call Obstacle on BeginPlay
  (CallFunction|SpawnRail))

(fn ConstructionScript)