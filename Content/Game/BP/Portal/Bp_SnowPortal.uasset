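; Portal actor that ends the snow world when BP_SnowPlayer overlaps its box and hands off to the next world.
; On overlap it plays a sound, shows a fade-to-black widget stored on the game instance, and immediately destroys the snow obstacles, game manager, killzones, gliders and coins.
; After a short delay it destroys the terrain generation and player, then calls ChangeWorld on the game instance, with its own lifespan set to expire shortly afterward.
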(event OnComponentBeginOverlap(Box)
  (params (OverlappedComponent :type Primitive%20Component%20Object%20Reference) (OtherActor :type Actor%20Object%20Reference) (OtherComp :type Primitive%20Component%20Object%20Reference) (OtherBodyIndex :type Integer) (bFromSweep :type Boolean) (SweepResult :type Hit%20Result%20Structure%20%28by%20ref%29))
  (Utilities|Casting|CastToBP_SnowPlayer OtherActor)
  (Audio|PlaySound2D "/Game/Game/Audio/SFX/going_through_portal.going_through_portal" 1.0 1.0 0.0 0 0)
  (bind _returnvalue (UserInterface|CreateWidget "/Game/Game/BP/UI/WBP_FadeToBlack.WBP_FadeToBlack_C"))
  (bind _asbp_game_instance (Utilities|Casting|CastTobp_GameInstance (Game|GetGameInstance)))
  (bind _output_get (Variables|/Game/Game/BP/bp_GameInstance.bp_GameInstance_C|SetFadeInOut _asbp_game_instance _returnvalue))
  (UserInterface|Viewport|AddtoViewport _output_get 0)
  (Utilities|FlowControl|Sequence
    (:then_0
      (bind _outactors (Actor|GetAllActorsOfClass "/Game/Game/BP/Obstacles/BP_SnowObstacle.BP_SnowObstacle_C"))
      (Actor|DestroyActor _outactors))
    (:then_1
      (bind _outactors_2 (Actor|GetAllActorsOfClass "/Game/Game/BP/Snow/BP_SnowGameManager.BP_SnowGameManager_C"))
      (Actor|DestroyActor _outactors_2))
    (:then_2
      (bind _outactors_3 (Actor|GetAllActorsOfClass "/Game/Game/BP/Snow/BP_SnowKillzone.BP_SnowKillzone_C"))
      (Actor|DestroyActor _outactors_3))
    (:then_3
      (bind _outactors_4 (Actor|GetAllActorsOfClass "/Game/Game/BP/PowerUps/BP_SnowGlider.BP_SnowGlider_C"))
      (Actor|DestroyActor _outactors_4))
    (:then_4
      (Actor|SetLifeSpan 3.0)
      (Utilities|FlowControl|Delay 2.0)
      (bind _outactors_5 (Actor|GetAllActorsOfClass "/Game/Game/BP/Snow/BP_SnowTerrainGeneration.BP_SnowTerrainGeneration_C"))
      (Actor|DestroyActor _outactors_5)
      (bind _returnvalue_2 (Actor|GetActorOfClass "/Game/Game/BP/Snow/BP_SnowPlayer.BP_SnowPlayer_C"))
      (Actor|DestroyActor _returnvalue_2)
      (bind _asbp_game_instance_2 (Utilities|Casting|CastTobp_GameInstance (Game|GetGameInstance)))
      (Default|ChangeWorld _asbp_game_instance_2))
    (:then_5
      (bind _outactors_6 (Actor|GetAllActorsOfClass "/Game/Game/BP/PowerUps/BP_Coin.BP_Coin_C"))
      (Actor|DestroyActor _outactors_6))))

(fn ConstructionScript)