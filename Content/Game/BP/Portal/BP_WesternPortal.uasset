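; Portal that takes the player out of the western level when a BP_Wagon overlaps its box.
; On overlap it plays a sound, adds a fade-to-black widget stored on the game instance, and immediately clears the manager, obstacles, generator and pickups.
; After a short delay it calls ChangeWorld on the game instance, then destroys the wagon, ground, rail generator, background and portal.
; The BP_Rail_Western cleanup is unconnected and never runs.
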(event OnComponentBeginOverlap(Box)
  (params (OverlappedComponent :type Primitive%20Component%20Object%20Reference) (OtherActor :type Actor%20Object%20Reference) (OtherComp :type Primitive%20Component%20Object%20Reference) (OtherBodyIndex :type Integer) (bFromSweep :type Boolean) (SweepResult :type Hit%20Result%20Structure%20%28by%20ref%29))
  (Utilities|Casting|CastToBP_Wagon OtherActor)
  (Actor|SetLifeSpan 2.0)
  (Audio|PlaySound2D "/Game/Game/Audio/SFX/going_through_portal.going_through_portal" 1.0 1.0 0.0 0 0)
  (bind _returnvalue (UserInterface|CreateWidget "/Game/Game/BP/UI/WBP_FadeToBlack.WBP_FadeToBlack_C"))
  (bind _asbp_game_instance (Utilities|Casting|CastTobp_GameInstance (Game|GetGameInstance)))
  (bind _output_get (Variables|/Game/Game/BP/bp_GameInstance.bp_GameInstance_C|SetFadeInOut _asbp_game_instance _returnvalue))
  (UserInterface|Viewport|AddtoViewport _output_get 0)
  (Utilities|FlowControl|Sequence
    (:then_0
      (bind _outactors (Actor|GetAllActorsOfClass "/Game/Game/BP/Western/BP_WesternManager.BP_WesternManager_C"))
      (Actor|DestroyActor _outactors))
    (:then_1
      (bind _outactors_2 (Actor|GetAllActorsOfClass "/Game/Game/BP/Obstacles/BP_ObstableGeneratorWesternLevel.BP_ObstableGeneratorWesternLevel_C"))
      (Actor|DestroyActor _outactors_2))
    (:then_2
      (bind _outactors_3 (Actor|GetAllActorsOfClass "/Game/Game/BP/Obstacles/bp_ObstacleWestern.bp_ObstacleWestern_C"))
      (Actor|DestroyActor _outactors_3))
    (:then_3
      (Actor|SetLifeSpan 3.0)
      (Utilities|FlowControl|Delay 2.0)
      (bind _asbp_game_instance_2 (Utilities|Casting|CastTobp_GameInstance (Game|GetGameInstance)))
      (Default|ChangeWorld _asbp_game_instance_2)
      (bind _outactors_4 (Actor|GetAllActorsOfClass "/Game/Game/BP/Western/BP_Wagon.BP_Wagon_C"))
      (Actor|DestroyActor _outactors_4)
      (bind _outactors_5 (Actor|GetAllActorsOfClass "/Game/Game/BP/Western/BP_GroundStartWesternLevel.BP_GroundStartWesternLevel_C"))
      (Actor|DestroyActor _outactors_5)
      (bind _outactors_6 (Actor|GetAllActorsOfClass "/Game/Game/BP/Western/BP_RailGeneratorLevelWestern.BP_RailGeneratorLevelWestern_C"))
      (Actor|DestroyActor _outactors_6)
      (bind _returnvalue_2 (Actor|GetActorOfClass "/Game/Game/BP/Western/BP_GroundGeneratorWestern.BP_GroundGeneratorWestern_C"))
      (Actor|DestroyActor _returnvalue_2)
      (bind _returnvalue_3 (Actor|GetActorOfClass "/Game/Game/BP/Western/BP_WesternBackground.BP_WesternBackground_C"))
      (Actor|DestroyActor _returnvalue_3)
      (bind _returnvalue_4 (Actor|GetActorOfClass "BP_WesternPortal_C"))
      (Actor|DestroyActor _returnvalue_4))
    (:then_4
      (bind _outactors_7 (Actor|GetAllActorsOfClass "/Game/Game/BP/PowerUps/BP_Lasso.BP_Lasso_C"))
      (Actor|DestroyActor _outactors_7))
    (:then_5
      (bind _outactors_8 (Actor|GetAllActorsOfClass "/Game/Game/BP/PowerUps/BP_Coin.BP_Coin_C"))
      (Actor|DestroyActor _outactors_8))
    (:then_6
      (bind _outactors_9 (Actor|GetAllActorsOfClass "/Game/Game/BP/PowerUps/BP_TNTobject.BP_TNTobject_C"))
      (Actor|DestroyActor _outactors_9))
    (:then_7
      (bind _outactors_10 (Actor|GetAllActorsOfClass "/Game/Game/BP/PowerUps/BP_RecupShield.BP_RecupShield_C"))
      (Actor|DestroyActor _outactors_10))))

(fn ConstructionScript)