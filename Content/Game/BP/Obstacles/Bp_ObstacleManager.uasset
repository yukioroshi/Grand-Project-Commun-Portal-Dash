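; Obstacle manager for the space level that spawns obstacles, power-ups, coins and a portal at four spawn points or its own position.
; Self-retriggering events drive each stream, with obstacle delays read from a time-based curve.
; Obstacles use single or paired points with random height offsets, rerolling repeat patterns.
; When the one-second countdown reaches zero, the obstacle loop spawns the portal above the manager, then destroys the manager.
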(event Custom|SpawnObstacle
  (bind _returnvalue (Transformation|GetActorTransform))
  (bind _obstacle (Variables|Default|GetObstacle))
  (bind _spawn1 (Variables|Default|GetSpawn1))
  (bind _spawn2 (Variables|Default|GetSPawn2))
  (bind _spawn3 (Variables|Default|GetSpawn3))
  (bind _spawn4 (Variables|Default|GetSpawn4))
  (bind _returnvalue_2 (Transformation|GetWorldTransform _spawn2))
  (bind (_location _rotation _scale) (Math|Transform|BreakTransform _returnvalue))
  (bind _returnvalue_3 (Transformation|GetWorldTransform _spawn3))
  (bind _returnvalue_4 (Transformation|GetWorldTransform _spawn1))
  (bind _returnvalue_5 (Transformation|GetWorldTransform _spawn4))
  (Utilities|FlowControl|Delay (Math|Curves|GetFloatValue (Variables|Default|GetSpawnDelay) (Utilities|Time|GetTimeSeconds)))
  (Variables|Default|SetselectedSPawn (Math|Random|RandomIntegerinRange 0 8))
  (if (== (Variables|Default|GetselectedSPawn) (Variables|Default|Getold%20spawn))
    (CallFunction|SpawnObstacle)
    (else
      (Variables|Default|Setold%20spawn (Variables|Default|GetselectedSPawn))
      (CallFunction|SpawnObstacle)
      (if (== (Variables|Default|GetTimer) 0)
        (Utilities|FlowControl|DoOnce false
          (:Completed
            (Game|SpawnActorfromClass "/Game/Game/BP/Portal/Bp_Portail.Bp_Portail_C" (Math|Transform|MakeTransform (+ _location "0.000000,0.000000,250.000000") _rotation _scale) "Undefined" "MultiplyWithRoot" 0 0)
            (Utilities|FlowControl|Delay 0.2)
            (Actor|DestroyActor)))
        (else
          (switch int (Variables|Default|GetselectedSPawn)
            (:0
              (Game|SpawnActorfromClass _obstacle (Math|Transform|MakeTransform (Math|Vector|MakeVector (.x (.location _returnvalue_4)) (.y (.location _returnvalue_4)) (+ (Math|Random|RandomFloatinRange -5e+01 5e+01) (.z (.location _returnvalue_4)))) (.rotation _returnvalue_4) (.scale _returnvalue_4)) "Undefined" "MultiplyWithRoot" 0 0 :!label _label))
            (:1
              (Game|SpawnActorfromClass _obstacle (Math|Transform|MakeTransform (Math|Vector|MakeVector (.x (.location _returnvalue_2)) (.y (.location _returnvalue_2)) (+ (Math|Random|RandomFloatinRange -5e+01 5e+01) (.z (.location _returnvalue_2)))) (.rotation _returnvalue_2) (.scale _returnvalue_2)) "Undefined" "MultiplyWithRoot" 0 0 :!label _label_2))
            (:2
              (Game|SpawnActorfromClass _obstacle (Math|Transform|MakeTransform (Math|Vector|MakeVector (.x (.location _returnvalue_3)) (.y (.location _returnvalue_3)) (+ (Math|Random|RandomFloatinRange -5e+01 5e+01) (.z (.location _returnvalue_3)))) (.rotation _returnvalue_3) (.scale _returnvalue_3)) "Undefined" "MultiplyWithRoot" 0 0 :!label _label_3))
            (:3
              (Game|SpawnActorfromClass _obstacle (Math|Transform|MakeTransform (Math|Vector|MakeVector (.x (.location _returnvalue_5)) (.y (.location _returnvalue_5)) (+ (Math|Random|RandomFloatinRange -5e+01 5e+01) (.z (.location _returnvalue_5)))) (.rotation _returnvalue_5) (.scale _returnvalue_5)) "Undefined" "MultiplyWithRoot" 0 0 :!label _label_4))
            (:4
              (Utilities|FlowControl|Sequence
                (:then_0
                  (goto _label_3))
                (:then_1
                  (goto _label_4))))
            (:5
              (Utilities|FlowControl|Sequence
                (:then_0
                  (goto _label))
                (:then_1
                  (goto _label_2))))
            (:6
              (Utilities|FlowControl|Sequence
                (:then_0
                  (goto _label_2))
                (:then_1
                  (goto _label_3))))
            (:7
              (Utilities|FlowControl|Sequence
                (:then_0
                  (goto _label_2))
                (:then_1
                  (goto _label_4))))
            (:8
              (Utilities|FlowControl|Sequence
                (:then_0
                  (goto _label))
                (:then_1
                  (goto _label_4))))))))))

(event Custom|Spawn%20PowerUp
  (bind _spawn1 (Variables|Default|GetSpawn1))
  (bind _spawn2 (Variables|Default|GetSPawn2))
  (bind _spawn3 (Variables|Default|GetSpawn3))
  (bind _spawn4 (Variables|Default|GetSpawn4))
  (bind _returnvalue (Transformation|GetWorldTransform _spawn2))
  (bind _returnvalue_2 (Transformation|GetWorldTransform _spawn3))
  (bind _returnvalue_3 (Transformation|GetWorldTransform _spawn4))
  (bind _returnvalue_4 (Transformation|GetWorldTransform _spawn1))
  ;[1 1 1] Génération Power Up Space Level
  (Utilities|FlowControl|Delay (Math|Random|RandomFloatinRange 1e+01 2e+01))
  (bind _output_get (Variables|Default|SetselectedSPawn (Math|Random|RandomIntegerinRange 0 3)))
  (switch int _output_get
    (:0
      (switch int (Math|Random|RandomIntegerinRange 0 2)
        (:0
          (Game|SpawnActorfromClass "/Game/Game/BP/PowerUps/Bp_Dash.Bp_Dash_C" _returnvalue_4 "Undefined" "MultiplyWithRoot" 0 200 0))
        (:1
          (Game|SpawnActorfromClass "/Game/Game/BP/PowerUps/BP_RecupShield.BP_RecupShield_C" _returnvalue_4 "Undefined" "MultiplyWithRoot" 0 0))
        (:2
          (Game|SpawnActorfromClass "/Game/Game/BP/PowerUps/BP_RecupLaser.BP_RecupLaser_C" _returnvalue_4 "Undefined" "MultiplyWithRoot" 0 0)))
      (CallFunction|SpawnPowerUp))
    (:1
      (switch int (Math|Random|RandomIntegerinRange 0 2)
        (:0
          (Game|SpawnActorfromClass "/Game/Game/BP/PowerUps/Bp_Dash.Bp_Dash_C" _returnvalue "Undefined" "MultiplyWithRoot" 0 200 0))
        (:1
          (Game|SpawnActorfromClass "/Game/Game/BP/PowerUps/BP_RecupLaser.BP_RecupLaser_C" _returnvalue "Undefined" "MultiplyWithRoot" 0 0))
        (:2
          (Game|SpawnActorfromClass "/Game/Game/BP/PowerUps/BP_RecupShield.BP_RecupShield_C" _returnvalue "Undefined" "MultiplyWithRoot" 0 0)))
      (CallFunction|SpawnPowerUp))
    (:2
      (switch int (Math|Random|RandomIntegerinRange 0 2)
        (:0
          (Game|SpawnActorfromClass "/Game/Game/BP/PowerUps/Bp_Dash.Bp_Dash_C" _returnvalue_2 "Undefined" "MultiplyWithRoot" 0 200 0))
        (:1
          (Game|SpawnActorfromClass "/Game/Game/BP/PowerUps/BP_RecupLaser.BP_RecupLaser_C" _returnvalue_2 "Undefined" "MultiplyWithRoot" 0 0))
        (:2
          (Game|SpawnActorfromClass "/Game/Game/BP/PowerUps/BP_RecupShield.BP_RecupShield_C" _returnvalue_2 "Undefined" "MultiplyWithRoot" 0 0)))
      (CallFunction|SpawnPowerUp))
    (:3
      (switch int (Math|Random|RandomIntegerinRange 0 2)
        (:0
          (Game|SpawnActorfromClass "/Game/Game/BP/PowerUps/Bp_Dash.Bp_Dash_C" _returnvalue_3 "Undefined" "MultiplyWithRoot" 0 200 0))
        (:1
          (Game|SpawnActorfromClass "/Game/Game/BP/PowerUps/BP_RecupLaser.BP_RecupLaser_C" _returnvalue_3 "Undefined" "MultiplyWithRoot" 0 0))
        (:2
          (Game|SpawnActorfromClass "/Game/Game/BP/PowerUps/BP_RecupShield.BP_RecupShield_C" _returnvalue_3 "Undefined" "MultiplyWithRoot" 0 0)))
      (CallFunction|SpawnPowerUp))))

(event Custom|Timer%20Portail
  ;[1 1 1] Timer Spawn Portail
  (bind _result (Math|Integer|DecrementInt (Variables|Default|GetTimer))
    (:%20%20
      (bind _output_get (Variables|Default|SetTimer _result))
      (if (== _output_get 0)
        (Utilities|FlowControl|Delay 5.0)
        (Variables|Default|SetTimer (Math|Random|RandomIntegerinRange 40 60))))))

(event Custom|Spawn%20Coin
  (Utilities|FlowControl|Delay (Math|Random|RandomFloatinRange 1.0 3.0))
  (bind _output_get (Variables|Default|SetselectedSPawn (Math|Random|RandomIntegerinRange 0 3)))
  (switch int _output_get
    (:0
      (Game|SpawnActorfromClass "/Game/Game/BP/PowerUps/BP_Coin.BP_Coin_C" (Transformation|GetWorldTransform (Variables|Default|GetSpawn1)) "Undefined" "MultiplyWithRoot" 0 0))
    (:1
      (Game|SpawnActorfromClass "/Game/Game/BP/PowerUps/BP_Coin.BP_Coin_C" (Transformation|GetWorldTransform (Variables|Default|GetSPawn2)) "Undefined" "MultiplyWithRoot" 0 0))
    (:2
      (Game|SpawnActorfromClass "/Game/Game/BP/PowerUps/BP_Coin.BP_Coin_C" (Transformation|GetWorldTransform (Variables|Default|GetSpawn3)) "Undefined" "MultiplyWithRoot" 0 0))
    (:3
      (Game|SpawnActorfromClass "/Game/Game/BP/PowerUps/BP_Coin.BP_Coin_C" (Transformation|GetWorldTransform (Variables|Default|GetSpawn4)) "Undefined" "MultiplyWithRoot" 0 0)))
  (CallFunction|SpawnCoin))

(event EventBeginPlay
  (CallFunction|SpawnObstacle)
  (CallFunction|SpawnPowerUp)
  (CallFunction|SpawnCoin)
  (Utilities|Time|SetTimerbyEvent (delegate Custom|Timer%20Portail) 1.0 true))

(fn ConstructionScript)