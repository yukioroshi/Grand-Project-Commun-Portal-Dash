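; BP_SnowObstacle is a snow level obstacle that randomly becomes a tree, snowman or logs on BeginPlay by enabling that mesh's visibility and collision.
; Touching the tree's overlap box has BP_SnowGameManager kill the player after a short delay.
; The snowman, checked once, destroys itself and stops a player whose Y velocity exceeds a threshold, otherwise kills them likewise.
; Logs only collide, with no overlap logic.
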(event OnComponentBeginOverlap(TreeBox)
  (params (OverlappedComponent :type Primitive%20Component%20Object%20Reference) (OtherActor :type Actor%20Object%20Reference) (OtherComp :type Primitive%20Component%20Object%20Reference) (OtherBodyIndex :type Integer) (bFromSweep :type Boolean) (SweepResult :type Hit%20Result%20Structure%20%28by%20ref%29))
  (Utilities|Casting|CastToBP_SnowPlayer OtherActor)
  (bind _returnvalue (Actor|GetActorOfClass "/Game/Game/BP/Snow/BP_SnowGameManager.BP_SnowGameManager_C"))
  (Utilities|FlowControl|Delay 0.2)
  (Default|ObstacleKillPlayer _returnvalue))

(event OnComponentBeginOverlap(SnowBox)
  (params (OverlappedComponent :type Primitive%20Component%20Object%20Reference) (OtherActor :type Actor%20Object%20Reference) (OtherComp :type Primitive%20Component%20Object%20Reference) (OtherBodyIndex :type Integer) (bFromSweep :type Boolean) (SweepResult :type Hit%20Result%20Structure%20%28by%20ref%29))
  (bind _asbp_snow_player (Utilities|Casting|CastToBP_SnowPlayer OtherActor))
  (Utilities|FlowControl|DoOnce false
    (:Completed
      (Development|PrintText (Utilities|Text|ToText(String) (Transformation|GetVelocity _asbp_snow_player)) true true "(R=1.000000,G=0.000000,B=0.186585,A=1.000000)" 15.0)
      (if (> (.Y (Math|Vector|BreakVector (Transformation|GetVelocity _asbp_snow_player))) 1.2e+03)
        (Physics|SetPhysicsLinearVelocity (Variables|/Game/Game/BP/Snow/BP_SnowPlayer.BP_SnowPlayer_C|Getportaldash_3d_snow_character _asbp_snow_player) "0, 0, 0" false "None")
        (Default|SpeedCheckWait _asbp_snow_player)
        (Actor|DestroyActor)
        (else
          (bind _returnvalue (Actor|GetActorOfClass "/Game/Game/BP/Snow/BP_SnowGameManager.BP_SnowGameManager_C"))
          (Utilities|FlowControl|Delay 0.2)
          (Default|ObstacleKillPlayer _returnvalue))))))

(event EventBeginPlay
  (bind _logs (Variables|Default|GetLogs))
  (bind _snowman (Variables|Default|GetSnowMan))
  (bind _tree (Variables|Default|GetTree))
  (switch int (Math|Random|RandomIntegerinRange 0 2)
    (:0
      (Variables|/Script/Engine.PrimitiveComponent|SetbGenerateOverlapEvents (Variables|Default|GetTreeBox) true)
      (Collision|SetCollisionEnabled _tree "QueryAndPhysics")
      (Rendering|SetVisibility _tree true false))
    (:1
      (Variables|/Script/Engine.PrimitiveComponent|SetbGenerateOverlapEvents (Variables|Default|GetSnowBox) true)
      (Collision|SetCollisionEnabled _snowman "QueryAndPhysics")
      (Rendering|SetVisibility _snowman true false))
    (:2
      (Collision|SetCollisionEnabled _logs "QueryAndPhysics")
      (Rendering|SetVisibility _logs true false))))

(fn ConstructionScript)