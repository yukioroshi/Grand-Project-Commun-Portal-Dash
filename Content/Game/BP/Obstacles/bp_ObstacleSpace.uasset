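; Asteroid obstacle that flies via ProjectileMovement, spins at a random rate, has a random scale and expires after a fixed lifespan.
; The construction script adds randomized speed scaled by the Speed curve sampled at game time.
; Hitting BP_Spaceship marks it not alive and triggers impact audio plus a timeline-driven scale shake.
; Delayed steps then play the death sound, fade to black and show the end screen.
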(event OnComponentHit(Cube)
  (params (HitComponent :type Primitive%20Component%20Object%20Reference) (OtherActor :type Actor%20Object%20Reference) (OtherComp :type Primitive%20Component%20Object%20Reference) (NormalImpulse :type Vector :default "0, 0, 0") (Hit :type Hit%20Result%20Structure%20%28by%20ref%29))
  ;[1 1 1] Hit player
  (bind _asbp_spaceship (Utilities|Casting|CastToBP_Spaceship OtherActor))
  (Variables|/Game/Game/BP/Space/BP_Spaceship.BP_Spaceship_C|SetIsAlive _asbp_spaceship false)
  (CallFunction|DestroyAsteroid)
  (Utilities|FlowControl|Delay 1.0)
  (Audio|PlaySound2D "/Game/Game/Audio/SFX/mort.mort" 1.0 1.0 0.0 0 0)
  (bind _returnvalue (Game|ConstructObjectfromClass "/Game/Game/BP/UI/WBP_FadeToBlack.WBP_FadeToBlack_C"))
  (UserInterface|Viewport|AddtoViewport _returnvalue 0)
  (Utilities|FlowControl|Delay 1.0)
  (bind _returnvalue_2 (UserInterface|CreateWidget "/Game/Game/BP/UI/UI_EndScreen.UI_EndScreen_C"))
  (UserInterface|Viewport|AddtoViewport _returnvalue_2 0))

(event Custom|Destroy%20Asteroid
  (Audio|Components|Audio|Play (Variables|Default|GetAudio) 0.0)
  (Variables|Default|SetPlayerDead true)
  (bind _shakealpha (Timeline|ImpactShake Play)
    (:Update
      (Transformation|SetRelativeScale3D (Variables|Default|GetDefaultSceneRoot) (Math|Conversions|ToVector(Float) _shakealpha)))))

(event EventBeginPlay
  (bind _returnvalue (Math|Random|RandomFloatinRange 1.0 2.0))
  ;[1 1 1] Init
  (Actor|SetLifeSpan 6.0)
  (Transformation|SetWorldScale3D (Variables|Default|GetCube) (Math|Vector|MakeVector _returnvalue _returnvalue _returnvalue))
  (Variables|/Script/Engine.RotatingMovementComponent|SetRotationRate (Variables|Default|GetRotatingMovement) (Math|Rotator|MakeRotator (Math|Random|RandomFloatinRange -1.8e+02 1.8e+02) 0.0 0.0)))

(fn ConstructionScript
  (bind _projectilemovement (Variables|Default|GetProjectileMovement))
  (Variables|/Script/Engine.ProjectileMovementComponent|SetMaxSpeed _projectilemovement (+ (Variables|/Script/Engine.ProjectileMovementComponent|GetMaxSpeed _projectilemovement) (* (Math|Curves|GetFloatValue (Variables|Default|GetSpeed) (Utilities|Time|GetTimeSeconds)) (Math|Random|RandomFloatinRange 1.5e+02 2e+02))))
  (Variables|/Script/Engine.ProjectileMovementComponent|SetInitialSpeed _projectilemovement (+ (Variables|/Script/Engine.ProjectileMovementComponent|GetMaxSpeed _projectilemovement) (* (Math|Curves|GetFloatValue (Variables|Default|GetSpeed) (Utilities|Time|GetTimeSeconds)) (Math|Random|RandomFloatinRange 1.5e+02 2e+02)))))