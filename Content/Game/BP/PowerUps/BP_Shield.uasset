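; BP_Shield is a timed power-up shield that absorbs one obstacle hit across the space, snow and western levels.
; On spawn it plays a shield sound and registers with bp_GameInstance's power-up UI, then a looping one-second timer counts down its duration.
; A sphere overlap destroys the obstacle and the shield with a break sound.
; Expiry also destroys it, and the Destroyed event notifies the game instance.
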(event OnComponentBeginOverlap(Sphere)
  (params (OverlappedComponent :type Primitive%20Component%20Object%20Reference) (OtherActor :type Actor%20Object%20Reference) (OtherComp :type Primitive%20Component%20Object%20Reference) (OtherBodyIndex :type Integer) (bFromSweep :type Boolean) (SweepResult :type Hit%20Result%20Structure%20%28by%20ref%29))
  ;[1 1 1] Collision Obstacle
  (Utilities|FlowControl|Sequence
    (:then_0
      (bind _asbp_obstacle_space (Utilities|Casting|CastTobp_ObstacleSpace OtherActor))
      (Utilities|IsValid _asbp_obstacle_space
        (:Is%20Valid
          (Actor|DestroyActor _asbp_obstacle_space))))
    (:then_1
      (bind _asbp_snow_obstacle (Utilities|Casting|CastToBP_SnowObstacle OtherActor))
      (Utilities|IsValid _asbp_snow_obstacle
        (:Is%20Valid
          (Actor|DestroyActor _asbp_snow_obstacle))))
    (:then_2
      (bind _asbp_obstacle_western (Utilities|Casting|CastTobp_ObstacleWestern OtherActor))
      (Utilities|IsValid _asbp_obstacle_western
        (:Is%20Valid
          (Actor|DestroyActor _asbp_obstacle_western)))))
  (Audio|Components|Audio|Stop (Variables|Default|GetAudioShield))
  (Audio|PlaySound2D "/Game/Game/Audio/SFX/shield_détruit.shield_détruit" 1.0 1.0 0.0 0 0)
  (bind _asbp_game_instance (Utilities|Casting|CastTobp_GameInstance (Game|GetGameInstance)))
  (Default|PowerUpDone _asbp_game_instance)
  (Actor|DestroyActor))

(event Custom|Timer
  ;[1 1 1] Timer
  (bind _result (Math|Integer|DecrementInt (Variables|Default|GetTime))
    (:%20%20
      (bind _output_get (Variables|Default|SetTime _result))
      (Default|UpdatePowerUpTime (Variables|Default|GetGameInstance) _output_get)
      (if (== _output_get 0)
        (Audio|Components|Audio|Stop (Variables|Default|GetAudioShield))
        (Actor|DestroyActor)))))

(event EventBeginPlay
  ;[1 1 1] Init bouclier
  (bind _returnvalue (Audio|SpawnSound2D "/Game/Game/Audio/SFX/shield_actif_new_version_2.shield_actif_new_version_2" 1.0 1.0 0.0 0))
  (Variables|Default|SetAudioShield _returnvalue)
  (bind _returnvalue_2 (Actor|GetActorOfClass "/Game/Game/BP/Snow/BP_SnowPlayer.BP_SnowPlayer_C"))
  (Variables|Default|SetSnow _returnvalue_2)
  (bind _returnvalue_3 (Actor|GetActorOfClass "/Game/Game/BP/Western/BP_Wagon.BP_Wagon_C"))
  (Variables|Default|SetWestern _returnvalue_3)
  (bind _returnvalue_4 (Actor|GetActorOfClass "/Game/Game/BP/Space/BP_Spaceship.BP_Spaceship_C"))
  (Variables|Default|SetSpace _returnvalue_4)
  (Utilities|FlowControl|Sequence
    (:then_0
      (bind _asbp_game_instance (Utilities|Casting|CastTobp_GameInstance (Game|GetGameInstance)))
      (bind _output_get (Variables|Default|SetGameInstance _asbp_game_instance))
      (Default|PowerUpUI _output_get 0 (Variables|Default|GetTime)) ; PowerUp = \n0=Shield\n1=Laser\n2=Wine\n3=Glider\n4=Lasso
    )
    (:then_1
      (Utilities|Time|SetTimerbyEvent (delegate Custom|Timer) 1.0 true))))

(event EventDestroyed
  ;[1 1 1] Hide HUD if PowerUp is done sooner
  (bind _asbp_game_instance (Utilities|Casting|CastTobp_GameInstance (Game|GetGameInstance)))
  (Default|PowerUpDone _asbp_game_instance))

(fn ConstructionScript)